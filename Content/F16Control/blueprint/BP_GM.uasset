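; BP_GM, apparently the game mode for an F16 control project, spawns the player's pilot at level start and shows control hints.
; On BeginPlay it gathers PlayerStart actors, destroys any pawn already held by the first player controller, then spawns BP_Pilot at the first start point and possesses it.
; It also prints timed on-screen messages describing the speed and yaw keys.
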(event Custom|spawnPlayer
  (bind _returnvalue (Game|GetPlayerController 0))
  (bind _startpoints (Variables|Default|GetstartPoints))
  (bind _returnvalue_2 (Pawn|GetControlledPawn _returnvalue))
  (bind _output (Utilities|Array|Get(acopy) _startpoints))
  (bind _outactors (Actor|GetAllActorsOfClass "/Script/Engine.PlayerStart"))
  (for _array_element _outactors
    (Utilities|Array|AddUnique (Variables|Default|GetstartPoints) _array_element))
  (Utilities|IsValid _output
    (:Is%20Valid
      (Utilities|IsValid _returnvalue_2
        (:Is%20Valid
          (Actor|DestroyActor _returnvalue_2))
        (:Is%20Not%20Valid
          _))
      (bind _returnvalue_3 (Game|SpawnActorfromClass "/Game/F16Control/blueprint/BP_Pilot.BP_Pilot_C" (Transformation|GetActorTransform _output) "AdjustIfPossibleButAlwaysSpawn" "OverrideRootScale" 0 0))
      (Pawn|Possess _returnvalue _returnvalue_3))))

(event EventBeginPlay
  (CallFunction|SpawnPlayer)
  (Development|PrintString "Right shift + Spacebar to control speed" true true "(R=1.000000,G=0.891900,B=0.000000,A=1.000000)" 3e+01)
  (Development|PrintString "Q + E keys to control yaw" true true "(R=1.000000,G=0.414395,B=0.000000,A=1.000000)" 3e+01))

(fn ConstructionScript)