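; BP_rocket is a self-propelled rocket projectile that flies along its local X axis and expires after 30 seconds.
; Each tick SetSpeed ramps speed toward MaxSpeed at a rate that grows with current speed, then applies a swept local offset.
; A Sphere overlap hides the Rocket component, spawns scaled effects and attenuated sound, then destroys the actor after a delay.
; The explosion applies no damage and does not stop movement.
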(event OnComponentBeginOverlap(Sphere)
  (params (OverlappedComponent :type Primitive%20Component%20Object%20Reference) (OtherActor :type Actor%20Object%20Reference) (OtherComp :type Primitive%20Component%20Object%20Reference) (OtherBodyIndex :type Integer) (bFromSweep :type Boolean) (SweepResult :type Hit%20Result%20Structure%20%28by%20ref%29))
  (CallFunction|Explosdion))

(event Custom|Explosdion
  (bind _returnvalue (Transformation|GetActorLocation))
  (Rendering|SetVisibility (Variables|Default|Getrocket) false false)
  (Effects|SpawnEmitteratLocation 0 _returnvalue "0, 0, 0" "10.000000,10.000000,10.000000")
  (Audio|SpawnSoundatLocation "/Game/F16Control/Cues/S_Explosion_Cue.S_Explosion_Cue" _returnvalue "0, 0, 0" 2.0 1.0 0.0 "/Game/F16Control/Cues/A_Attenuation.A_Attenuation" 0)
  (Utilities|FlowControl|Delay 5.0)
  (Actor|DestroyActor))

(event EventBeginPlay
  (Actor|SetLifeSpan 3e+01))

(event EventTick
  (params (DeltaSeconds :type Float%20%28single-precision%29))
  (CallFunction|SetSpeed DeltaSeconds))

(fn ConstructionScript)

(fn SetSpeed
  (params (deltaTime :type Float%20%28double-precision%29))
  (bind _maxspeed (Variables|Default|GetmaxSpeed))
  (if (< (Variables|Default|GetcurrentSpeed) _maxspeed)
    (Variables|Default|SetcurrentSpeed (Math|Interpolation|FInterptoConstant (Variables|Default|GetcurrentSpeed) _maxspeed deltaTime (* (+ (Math|Float|Absolute(Float) (/ (Variables|Default|GetcurrentSpeed) _maxspeed)) 1.0) (Variables|Default|GetSpeedInterp))))
    (else
      (Variables|Default|SetcurrentSpeed (Variables|Default|GetmaxSpeed))))
  (Transformation|AddActorLocalOffset (Math|Vector|MakeVector (* deltaTime (Variables|Default|GetcurrentSpeed)) 0.0 0.0) true false))